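; BP_Item_Stethoscope is a stethoscope item that detects which body point it is placed on.
; About every half second it capsule-traces down from its Cone, looking for a BP_point whose body side matches the GameMode's current side.
; A match prints the point's Id and sends it once through BP_GameInstance, re-armed when the trace hits another kind of actor.
; Events toggle its visibility and restore the Cone's starting location.
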(event Custom|ResetLocation
  (Transformation|SetWorldLocation (Variables|Default|GetCone) (Variables|Default|GetDefaultLocation) false false))

(event Custom|ShowStethoscope
  (params (bNewVisibility :type Boolean))
  (Rendering|SetActorHiddenInGame bNewVisibility))

(event EventBeginPlay
  (bind _asbp_game_instance (Utilities|Casting|CastToBP_GameInstance (Game|GetGameInstance)))
  (Variables|Default|SetGame%20Instance _asbp_game_instance)
  (Variables|Default|SetDefaultLocation (Transformation|GetWorldLocation (Variables|Default|GetCone)))
  (bind _asbp_game_mode (Utilities|Casting|CastToBP_GameMode (Game|GetGameMode)))
  (Variables|Default|SetGame%20Mode _asbp_game_mode))

(event EventTick
  (params (DeltaSeconds :type Float%20%28single-precision%29))
  (bind _cone (Variables|Default|GetCone))
  (bind _returnvalue (Transformation|GetWorldLocation _cone))
  (Utilities|FlowControl|Delay 0.5)
  (bind (_outhit _returnvalue_2) (Collision|CapsuleTraceByChannel _returnvalue (+ _returnvalue (* (* (Math|Vector|GetUpVector (Variables|Default|GetCone)) -1.0) 5e+02)) 5.0 5e+01 "TraceTypeQuery1" false 0 "None"))
  (if _returnvalue_2
    (bind _asbp_point (Utilities|Casting|CastToBP_point (.HitActor (Collision|BreakHitResult _outhit)))
      (:then
        (if (Utilities|Enum|Equal(Enum) (Variables|/Game/blueprints/BP_point.BP_point_C|GetBodySide _asbp_point) (Variables|/Game/blueprints/framework/BP_GameMode.BP_GameMode_C|GetCurrentBodySide (Variables|Default|GetGame%20Mode)))
          (Development|PrintString (Variables|/Game/blueprints/BP_point.BP_point_C|GetId _asbp_point) true true "(R=0.000000,G=0.660000,B=1.000000,A=1.000000)" 0.0)
          (Utilities|FlowControl|DoOnce false :!label _label
            (:Completed
              (Default|SendMessage (Variables|Default|GetGame%20Instance) (Variables|/Game/blueprints/BP_point.BP_point_C|GetId _asbp_point) "stethoscope")))))
      (:CastFailed
        (goto _label Reset)))))

(fn ConstructionScript)