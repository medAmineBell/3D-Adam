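; BP_point is a clickable body sensor point, identified by an Id and a body type such as pulse or capillary refill.
; It caches BP_GameInstance on BeginPlay; clicking Sphere1 prints the Id and type for debugging.
; The click then sends the Id through the GameInstance's SendMessage with a trigger matching the body type.
; Unconnected leftover branches show thumb-specific capillary refill checks keyed on Id.
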(event OnClicked(Sphere1)
  (params (TouchedComponent :type Primitive%20Component%20Object%20Reference) (ButtonPressed :type Key%20Structure :default "None"))
  (bind _bodytype (Variables|Default|GetbodyType))
  (Development|PrintString (Variables|Default|GetId))
  (Development|PrintString (Utilities|String|EnumtoString _bodytype))
  (switch Utilities|FlowControl|Switch|SwitchonBodyType _bodytype
    (:NewEnumerator4
      (Default|SendMessage (Variables|Default|GetGame%20Instance) (Variables|Default|GetId) "triggerPulse"))
    (:NewEnumerator9
      (Default|SendMessage (Variables|Default|GetGame%20Instance) (Variables|Default|GetId) "capillaryRefill"))))

(event EventBeginPlay
  (bind _asbp_game_instance (Utilities|Casting|CastToBP_GameInstance (Game|GetGameInstance)))
  (Variables|Default|SetGame%20Instance _asbp_game_instance))

(event Collision|EventActorBeginOverlap
  (params (OtherActor :type Actor%20Object%20Reference)))

(event EventTick
  (params (DeltaSeconds :type Float%20%28single-precision%29)))

(fn ConstructionScript)