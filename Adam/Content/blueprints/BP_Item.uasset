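; BP_Item is an item actor that starts following the mouse cursor when its static mesh is clicked.
; The click sets CanMove, which nothing in these graphs clears, and Tick then moves the actor each frame at a fixed height.
; X and Y come straight from the deprojected mouse world location, without a trace or use of the ray direction.
; Debug prints show the actor location every frame and the mouse world location on click.
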(event OnClicked(StaticMeshComponent0)
  (params (TouchedComponent :type Primitive%20Component%20Object%20Reference) (ButtonPressed :type Key%20Structure :default "None"))
  (Variables|Default|SetbCanMove true)
  (Development|PrintString (Utilities|String|ToString(Vector) (.WorldLocation (Game|Player|ConvertMouseLocationToWorldSpace (Game|GetPlayerController 0))))))

(event EventTick
  (params (DeltaSeconds :type Float%20%28single-precision%29))
  (bind _returnvalue (Game|GetPlayerController 0))
  (bind _worldlocation (Game|Player|ConvertMouseLocationToWorldSpace _returnvalue))
  (Development|PrintString (Utilities|String|ToString(Vector) (Transformation|GetActorLocation)) true true "(R=0.000000,G=0.660000,B=1.000000,A=1.000000)" 0.0)
  (if (Variables|Default|GetbCanMove)
    (Transformation|SetActorLocation (Math|Vector|MakeVector (.x _worldlocation) (.y _worldlocation) 1.3e+02) false false)))

(fn ConstructionScript)